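; GA_Aim is a gameplay ability that puts the player character into weapon aiming.
; On activation it calls Aim on the avatar's combat component and plays the AM_Aim montage through a wait task.
; Interruption or cancellation of the montage ends the ability, and ending it always calls UnAim on the combat component.
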(event `self.K2_ActivateAbility`
  (bind _combatcomponent (`ChronoPlayerCharacter.CombatComponent` (cast `/Game/Blueprints/Characters/Player/BP_PlayerCharacter` (`self.GetAvatarActorFromActorInfo`) :!pure true)))
  (`parent.K2_ActivateAbility`)
  (`CombatComponent.Aim` _combatcomponent)
  (set `self.Combat Component` _combatcomponent)
  (`AbilityTask_PlayMontageAndWait.CreatePlayMontageAndWaitProxy` "None" "/Game/Blueprints/Animation/Montages/AM_Aim.AM_Aim"
    (:`OnInterrupted`
      _)
    (:`OnCancelled`
      _))
  (`self.K2_EndAbility`))

(event `self.K2_OnEndAbility`
  (params (bWasCancelled :type Boolean))
  (`parent.K2_OnEndAbility` bWasCancelled)
  (`CombatComponent.UnAim` (`self.Combat Component`)))